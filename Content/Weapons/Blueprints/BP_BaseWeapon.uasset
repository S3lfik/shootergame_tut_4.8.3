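; Base weapon Blueprint that tracks magazine and backpack ammo, bullet spread and shot aiming.
; Fire only decrements the magazine; Reload refills it from the backpack without crediting rounds left in it.
; CalculateShootInformations traces from the camera within the spread cone, returning a muzzle-socket projectile transform, hit and end point, with persistent debug drawing.
; Spread increases through clamped calls and recovers toward its minimum on Tick.
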(event EventBeginPlay
  (Variables|Default|SetCurrentAmmoInMag%20 (Variables|Default|GetMaxAmmoInMag%20))
  (Variables|Default|SetCurrentAmmoInBackpack (Variables|Default|GetMaxAmmoInBackpack)))

(event Collision|EventActorBeginOverlap
  (params (OtherActor :type Actor%20Object%20Reference)))

(event EventTick
  (params (DeltaSeconds :type Float%20%28single-precision%29))
  (Variables|Default|SetDeltaTime DeltaSeconds)
  (if (> (Variables|Default|GetSpreadCurrent) (Variables|Default|GetSpreadMin))
    (CallFunction|DecreaseSpread (* (Variables|Default|GetDeltaTime) (Variables|Default|GetSpreadDecreaseSpeed)))))

(fn ConstructionScript)

(fn Fire
  (Variables|Default|SetCurrentAmmoInMag%20 (- (Variables|Default|GetCurrentAmmoInMag%20) 1)))

(fn Reload
  (Variables|Default|SetCurrentAmmoInMag%20 (Math|Integer|Min(Integer) (Variables|Default|GetMaxAmmoInMag%20) (Variables|Default|GetCurrentAmmoInBackpack)))
  (Variables|Default|SetCurrentAmmoInBackpack (- (Variables|Default|GetCurrentAmmoInBackpack) (Math|Integer|Min(Integer) (Variables|Default|GetMaxAmmoInMag%20) (Variables|Default|GetCurrentAmmoInBackpack)))))

(fn HaveAmmoinMag
  (return (> (Variables|Default|GetCurrentAmmoInMag%20) 0) (== (Variables|Default|GetCurrentAmmoInMag%20) (Variables|Default|GetMaxAmmoInMag%20))))

(fn HaveAmmoinBackpack
  (return (> (Variables|Default|GetCurrentAmmoInBackpack) 0)))

(fn CalculateShootInformations
  (params (Camera :type Camera%20Component%20Object%20Reference) (WeaponMesh :type Scene%20Component%20Object%20Reference) (WeaponFireSocketName :type Name))
  (Utilities|FlowControl|Sequence
    (:then_0
      (LocalVariables|SetLocalCamera Camera)
      (LocalVariables|SetLocalWeaponMesh WeaponMesh)
      (LocalVariables|SetLocalWeaponSocketName WeaponFireSocketName))
    (:then_1
      (LocalVariables|SetLocalEndLoc (+ (* (Class|KismetMathLibrary|RandomUnitVectorinCone (Math|Vector|GetForwardVector (.rotation (Transformation|GetWorldTransform (LocalVariables|GetLocalCamera)))) (Variables|Default|GetSpreadCurrent)) (Variables|Default|GetLineTraceLength)) (.location (Transformation|GetWorldTransform (LocalVariables|GetLocalCamera)))))
      (bind (_outhit _returnvalue) (Collision|LineTraceByChannel (.location (Transformation|GetWorldTransform (LocalVariables|GetLocalCamera))) (+ (* (Class|KismetMathLibrary|RandomUnitVectorinCone (Math|Vector|GetForwardVector (.rotation (Transformation|GetWorldTransform (LocalVariables|GetLocalCamera)))) (Variables|Default|GetSpreadCurrent)) (Variables|Default|GetLineTraceLength)) (.location (Transformation|GetWorldTransform (LocalVariables|GetLocalCamera)))) "TraceTypeQuery1" false 0 "Persistent"))
      (if _returnvalue
        (LocalVariables|SetLocalTransform (Math|Transform|MakeTransform (Transformation|GetSocketLocation (LocalVariables|GetLocalWeaponMesh) (LocalVariables|GetLocalWeaponSocketName)) (Math|Rotator|FindLookatRotation (.ImpactPoint (Collision|BreakHitResult _outhit)) (Transformation|GetSocketLocation (LocalVariables|GetLocalWeaponMesh) (LocalVariables|GetLocalWeaponSocketName)))))
        (LocalVariables|SetLocalEndLoc (.ImpactPoint (Collision|BreakHitResult _outhit)))
        (else
          (bind _aspawn (Utilities|Casting|CastToPawn (Components|GetOwner (LocalVariables|GetLocalCamera))))
          (LocalVariables|SetLocalTransform (Math|Transform|MakeTransform (Transformation|GetSocketLocation (LocalVariables|GetLocalWeaponMesh) (LocalVariables|GetLocalWeaponSocketName)) (Pawn|GetControlRotation _aspawn :!class /Script/Engine.Pawn))))))
    (:then_2
      (return (LocalVariables|GetLocalTransform) _outhit (LocalVariables|GetLocalEndLoc)))))

(fn IncreaseSpread
  (params (Amount :type Float%20%28single-precision%29))
  (if (>= (+ Amount (Variables|Default|GetSpreadCurrent)) (Variables|Default|GetSpreadMax))
    (Variables|Default|SetSpreadCurrent (Variables|Default|GetSpreadMax))
    (else
      (Variables|Default|SetSpreadCurrent (+ Amount (Variables|Default|GetSpreadCurrent))))))

(fn DecreaseSpread
  (params (Amount :type Float%20%28single-precision%29))
  (if (<= (- (Variables|Default|GetSpreadCurrent) Amount) (Variables|Default|GetSpreadMin))
    (Variables|Default|SetSpreadCurrent (Variables|Default|GetSpreadMin))
    (else
      (Variables|Default|SetSpreadCurrent (- (Variables|Default|GetSpreadCurrent) Amount)))))