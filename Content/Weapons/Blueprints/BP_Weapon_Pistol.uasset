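; Pistol weapon Blueprint that extends a parent weapon's fire and reload behavior.
; On BeginPlay it takes its ammo data from the conventional ammo entry in ShooterGameInstance and sets spread and damage modifier ranges, starting at maximum spread.
; Firing runs the parent logic, then plays the pistol mesh animation, spawns a shell effect at the AmmoSocket and increases spread.
; Reload defers entirely to the parent.
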(event EventBeginPlay
  (|CallParentFunction)
  (bind _asshooter_game_instance (Utilities|Casting|CastToShooterGameInstance (Game|GetGameInstance))
    (:then
      (Variables|Default|SetAmmoData (Variables|/Game/GameFiles/ShooterGameInstance.ShooterGameInstance_C|GetAmmo_Convetional _asshooter_game_instance)))
    (:CastFailed
      _))
  (Variables|Default|SetSpreadMin 0.0)
  (bind _output_get (Variables|Default|SetSpreadMax 0.3))
  (Variables|Default|SetSpreadCurrent _output_get)
  (Variables|Default|SetSpreadDecreaseSpeed 0.25)
  (Variables|Default|SetMinWeaponDamageModifier 0.8)
  (Variables|Default|SetMaxWeaponDamageModifier 1.2))

(event Collision|EventActorBeginOverlap
  (params (OtherActor :type Actor%20Object%20Reference)))

(event EventTick
  (params (DeltaSeconds :type Float%20%28single-precision%29)))

(event EventFire
  (bind _weaponmesh (Variables|Default|GetWeaponMesh))
  (bind _returnvalue (Transformation|GetSocketTransform _weaponmesh "AmmoSocket" "RTS_World"))
  (|CallParentFunction)
  (Components|Animation|PlayAnimation (Variables|Default|GetWeaponMesh) "/Game/MilitaryWeapSilver/Weapons/Animations/Fire_Pistol_W.Fire_Pistol_W" false)
  (Effects|SpawnEmitteratLocation "/Game/Weapons/FX/FX_Shell_Pistol.FX_Shell_Pistol" (.location _returnvalue) (.rotation _returnvalue))
  (CallFunction|IncreaseSpread 0.1))

(event EventReload
  (|CallParentFunction))

(fn ConstructionScript
  (|CallParentFunction))