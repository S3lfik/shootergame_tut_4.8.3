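; Base enemy actor that tracks health, takes weapon damage and removes itself shortly after death.
; TakeDamage scales ammo damage by a random weapon modifier, a crit roll and the hit physical material's DestructibleDamageThresholdScale, repurposed as a damage multiplier.
; The result reduces health and updates the debug health bar widget.
; Non-lethal hits spawn a short-lived DamageFeedback actor at the impact point, showing damage and crit state.
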(event EventBeginPlay
  (bind _output_get (Variables|Default|SetMaxHealth 1e+02))
  (Variables|Default|SetCurrentHealth _output_get))

(event Collision|EventActorBeginOverlap
  (params (OtherActor :type Actor%20Object%20Reference)))

(event EventTick
  (params (DeltaSeconds :type Float%20%28single-precision%29)))

(event EventTakeDamage
  (params (AmmoData :type Ammo%20Data%20Structure) (MinWeaponDmgModifier :type Float%20%28single-precision%29) (MaxWeaponDmgModifier :type Float%20%28single-precision%29) (CritDmgModifier :type Float%20%28single-precision%29) (DamageCauser :type Actor%20Object%20Reference) (HitInfo :type Hit%20Result%20Structure))
  (bind (_ammotype _damage _critchance) (Utilities|Struct|BreakAmmoData AmmoData))
  (if (not (Variables|Default|GetisDead))
    (bind (_wascrit _damagetaken) (CallFunction|CalculateDamage _damage _critchance CritDmgModifier (Math|Random|RandomFloatinRange MinWeaponDmgModifier MaxWeaponDmgModifier) HitInfo))
    (bind _isdead (CallFunction|ModifyHealt _damagetaken))
    (bind _output_get (Variables|Default|SetisDead _isdead))
    (if _output_get
      (Actor|SetLifeSpan 0.1)
      (else
        (bind _returnvalue (Game|SpawnActorfromClass "/Game/Weapons/Data/DamageFeedback.DamageFeedback_C" (Math|Transform|MakeTransform (.ImpactPoint (Collision|BreakHitResult HitInfo)) "0, 0, 0" "1,1,1") false 0 _damagetaken _wascrit))
        (Actor|SetLifeSpan _returnvalue 1.0)))))

(fn ConstructionScript)

(fn UpdateHealthBar
  (bind _asui_debug_enemy_health (Utilities|Casting|CastToUI_Debug_EnemyHealth (UserInterface|GetUserWidgetObject (Variables|Default|GetHealthBar))))
  (Default|UpdateHealthBar _asui_debug_enemy_health (Variables|Default|GetCurrentHealth) (Variables|Default|GetMaxHealth)))

(fn ModifyHealt
  (params (delta :type Float%20%28single-precision%29))
  (Utilities|FlowControl|Sequence
    (:then_0
      (if (>= delta (Variables|Default|GetCurrentHealth))
        (Variables|Default|SetisDead true)
        (Variables|Default|SetCurrentHealth 0.0)
        (else
          (Variables|Default|SetisDead false)
          (Variables|Default|SetCurrentHealth (- (Variables|Default|GetCurrentHealth) delta)))))
    (:then_1
      (CallFunction|UpdateHealthBar)
      (return (Variables|Default|GetisDead)))))

(fn CalculateDamage
  (params (damage :type Float%20%28single-precision%29) (critChance :type Float%20%28single-precision%29) (critDmgModifier :type Float%20%28single-precision%29) (weaponDmgModifier :type Float%20%28single-precision%29) (HitInfo :type Hit%20Result%20Structure))
  (LocalVariables|Setl_currentDamage%20 (* damage weaponDmgModifier))
  (Utilities|FlowControl|Sequence
    (:then_0
      (bind _output_get (LocalVariables|Setl_wasCrit (< (Math|Random|RandomFloatinRange 0.0 1e+02) critChance)))
      (if _output_get
        (LocalVariables|Setl_currentDamage%20 (* (LocalVariables|Getl_currentDamage%20) critDmgModifier))))
    (:then_1
      (LocalVariables|Setl_currentDamage%20 (* (LocalVariables|Getl_currentDamage%20) (Variables|/Script/Engine.PhysicalMaterial|GetDestructibleDamageThresholdScale (.PhysMat (Collision|BreakHitResult HitInfo))))))
    (:then_2
      (return (LocalVariables|Getl_wasCrit) (LocalVariables|Getl_currentDamage%20)))))